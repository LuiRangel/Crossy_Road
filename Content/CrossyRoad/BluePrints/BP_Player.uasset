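; BP_Player is the player pawn for a Crossy Road-style game, moved by discrete key presses.
; Forward, back, left and right action presses add movement input along the actor's axes, scaled by Units.
; Tick consumes that vector and applies it as an unswept local offset times delta seconds, so each press's distance depends on frame time.
; Axis-based movement and a mesh rotation remain as unconnected nodes.
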(event EventBeginPlay)

(event Collision|EventActorBeginOverlap
  (params (OtherActor :type Actor%20Object%20Reference)))

(event EventTick
  (params (DeltaSeconds :type Float%20%28single-precision%29))
  (bind _returnvalue (Class|Pawn|ConsumeMovementInputVector))
  (Transformation|AddActorLocalOffset (* _returnvalue DeltaSeconds) false false))

(event Input|ActionEvents|InputActionMoveFoward
  (params (Key :type Key%20Structure))
  (:Pressed
    (Pawn|Input|AddMovementInput (Transformation|GetActorForwardVector) (Variables|Default|GetUnits) false)))

(event Input|ActionEvents|InputActionMoveRight
  (params (Key :type Key%20Structure))
  (:Pressed
    (Pawn|Input|AddMovementInput (Transformation|GetActorRightVector) (Variables|Default|GetUnits) false)))

(event Input|ActionEvents|InputActionMoveLeft
  (params (Key :type Key%20Structure))
  (:Pressed
    (Pawn|Input|AddMovementInput (Transformation|GetActorRightVector) (* -1 (Variables|Default|GetUnits)) false)))

(event Input|ActionEvents|InputActionMoveBack
  (params (Key :type Key%20Structure))
  (:Pressed
    (Pawn|Input|AddMovementInput (Transformation|GetActorForwardVector) (* -1 (Variables|Default|GetUnits)) false)))

(event Input|AxisEvents|InputAxisMoveFoward
  (params (AxisValue :type Float%20%28single-precision%29)))

(event Input|AxisEvents|InputAxisMoveRight
  (params (AxisValue :type Float%20%28single-precision%29)))

(fn ConstructionScript)