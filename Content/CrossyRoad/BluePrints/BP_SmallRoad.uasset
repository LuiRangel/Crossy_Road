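; Road lane for a Crossy Road-style game that sends cars and trucks across in one random direction.
; BeginPlay picks direction and a shared speed; a Delay on Tick acts as a random spawn timer.
; SpawnCar and SpawnTruck add vehicles as child actors at the matching side, favoring cars.
; End triggers destroy BP_Car actors, and player overlap with Triggerzone tells GroundSpawner to spawn the next lane.
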(event OnComponentBeginOverlap(Triggerzone)
  (params (OverlappedComponent :type Primitive%20Component%20Object%20Reference) (OtherActor :type Actor%20Object%20Reference) (OtherComp :type Primitive%20Component%20Object%20Reference) (OtherBodyIndex :type Integer) (bFromSweep :type Boolean) (SweepResult :type Hit%20Result%20Structure%20%28by%20ref%29))
  ;[1 1 1] Spawn next lane if triggerzone is triggered
  (Utilities|Casting|CastToBP_Player OtherActor)
  (Default|SpawnatSpawnPoint (Variables|Default|GetGroundSpawner)))

(event OnComponentBeginOverlap(LeftTeleporter)
  (params (OverlappedComponent :type Primitive%20Component%20Object%20Reference) (OtherActor :type Actor%20Object%20Reference) (OtherComp :type Primitive%20Component%20Object%20Reference) (OtherBodyIndex :type Integer) (bFromSweep :type Boolean) (SweepResult :type Hit%20Result%20Structure%20%28by%20ref%29))
  ;[1 1 1] Check Leftside Car Trigger
  (bind _asbp_car (Utilities|Casting|CastToBP_Car OtherActor))
  (if (Variables|Default|GetLeftBound)
    (Actor|DestroyActor _asbp_car)))

(event OnComponentBeginOverlap(RightTeleporter)
  (params (OverlappedComponent :type Primitive%20Component%20Object%20Reference) (OtherActor :type Actor%20Object%20Reference) (OtherComp :type Primitive%20Component%20Object%20Reference) (OtherBodyIndex :type Integer) (bFromSweep :type Boolean) (SweepResult :type Hit%20Result%20Structure%20%28by%20ref%29))
  ;[1 1 1] Check Rightside Car Trigger
  (bind _asbp_car (Utilities|Casting|CastToBP_Car OtherActor))
  (if (Variables|Default|GetRightBound)
    (Actor|DestroyActor _asbp_car)))

(event EventBeginPlay
  ;[1 1 1] Decides where the car is coming from
  (if (<= (Math|Random|RandomIntegerinRange 0 100) 50)
    (Variables|Default|SetLeftBound true) ; Car spawns on the right
    (Variables|Default|SetVehicle%20Speed (Math|Random|RandomFloatinRange 3e+02 4.5e+02))
    (else
      (Variables|Default|SetRightBound true) ; Car spawns on the left
      (Variables|Default|SetVehicle%20Speed (Math|Random|RandomFloatinRange 3e+02 4.5e+02)))))

(event EventTick
  (params (DeltaSeconds :type Float%20%28single-precision%29))
  ;[1 1 1] Spawn Vehicle, set scale, location, speed, and direction.
  (Utilities|FlowControl|Delay (Math|Random|RandomFloatinRange 0.25 3.0))
  (if (<= (Math|Random|RandomFloatinRange 0.0 1.0) 0.6)
    (CallFunction|SpawnCar)
    (else
      (CallFunction|SpawnTruck))))

(fn ConstructionScript)

(fn SpawnCar
  (bind _returnvalue (AddComponent|AddChildActorComponent false))
  (bind _asbp_car (Utilities|Casting|CastToBP_Car (Variables|/Script/Engine.ChildActorComponent|GetChildActor _returnvalue)))
  (if (Variables|Default|GetLeftBound)
    (Variables|/Game/CrossyRoad/BluePrints/BP_Car.BP_Car_C|SetSpeed _asbp_car (Variables|Default|GetVehicle%20Speed)) ; might not work with concurrent cars idk
    (Transformation|SetWorldTransform _returnvalue (Math|Transform|MakeTransform (Transformation|GetWorldLocation (Variables|Default|GetRightSpawn)) "0.000000,180.000000,0.000000" "1,1,1") false false)
    (else
      (Variables|/Game/CrossyRoad/BluePrints/BP_Car.BP_Car_C|SetSpeed _asbp_car (Variables|Default|GetVehicle%20Speed))
      (Transformation|SetWorldLocation _returnvalue (Transformation|GetWorldLocation (Variables|Default|GetLeftSpawn)) false false)
      (Transformation|SetWorldScale3D _returnvalue "1.000000,1.000000,1.000000"))))

(fn SpawnTruck
  (bind _returnvalue (AddComponent|AddChildActorComponent false))
  (bind _asbp_truck (Utilities|Casting|CastToBP_Truck (Variables|/Script/Engine.ChildActorComponent|GetChildActor _returnvalue)))
  (if (Variables|Default|GetLeftBound)
    (Variables|/Game/CrossyRoad/BluePrints/BP_Truck.BP_Truck_C|SetSpeed _asbp_truck (Variables|Default|GetVehicle%20Speed))
    (Transformation|SetWorldTransform _returnvalue (Math|Transform|MakeTransform (Transformation|GetWorldLocation (Variables|Default|GetRightSpawn)) "0.000000,180.000000,0.000000" "1,1,1") false false)
    (Transformation|AddWorldOffset _returnvalue "0, 0,8.000000" false false)
    (else
      (Variables|/Game/CrossyRoad/BluePrints/BP_Truck.BP_Truck_C|SetSpeed _asbp_truck (Variables|Default|GetVehicle%20Speed))
      (Transformation|SetWorldLocation _returnvalue (Transformation|GetWorldLocation (Variables|Default|GetLeftSpawn)) false false)
      (Transformation|SetWorldScale3D _returnvalue "1.000000,1.000000,1.000000")
      (Transformation|AddWorldOffset _returnvalue "0, 0,8.000000" false false))))