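; River lane for a Crossy Road-style game that sends floating logs across in one randomly chosen direction at a random speed set on BeginPlay.
; A Delay on Tick acts as a random-interval timer, adding one of two log types as child actors at the upstream spawn point.
; Side teleporter overlaps destroy logs at the downstream end, while the player entering the trigger zone makes GroundSpawner spawn the next lane.
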(event OnComponentBeginOverlap(Triggerzone)
  (params (OverlappedComponent :type Primitive%20Component%20Object%20Reference) (OtherActor :type Actor%20Object%20Reference) (OtherComp :type Primitive%20Component%20Object%20Reference) (OtherBodyIndex :type Integer) (bFromSweep :type Boolean) (SweepResult :type Hit%20Result%20Structure%20%28by%20ref%29))
  ;[1 1 1] Spawn next lane if triggerzone is triggered
  (Utilities|Casting|CastToBP_Player OtherActor)
  (Default|SpawnatSpawnPoint (Variables|Default|GetGroundSpawner)))

(event OnComponentBeginOverlap(LeftTeleporter)
  (params (OverlappedComponent :type Primitive%20Component%20Object%20Reference) (OtherActor :type Actor%20Object%20Reference) (OtherComp :type Primitive%20Component%20Object%20Reference) (OtherBodyIndex :type Integer) (bFromSweep :type Boolean) (SweepResult :type Hit%20Result%20Structure%20%28by%20ref%29))
  ;[1 1 1] Check Leftside vehicle Trigger
  (bind _asbp_log_1 (Utilities|Casting|CastToBP_Log1 OtherActor)
    (:then
      (if (Variables|Default|GetLeftBound)
        (Actor|DestroyActor _asbp_log_1)))
    (:CastFailed
      (bind _asbp_log_2 (Utilities|Casting|CastToBP_Log2 OtherActor))
      (if (Variables|Default|GetLeftBound)
        (Actor|DestroyActor _asbp_log_2)))))

(event OnComponentBeginOverlap(RightTeleporter)
  (params (OverlappedComponent :type Primitive%20Component%20Object%20Reference) (OtherActor :type Actor%20Object%20Reference) (OtherComp :type Primitive%20Component%20Object%20Reference) (OtherBodyIndex :type Integer) (bFromSweep :type Boolean) (SweepResult :type Hit%20Result%20Structure%20%28by%20ref%29))
  ;[1 1 1] Check Rightside vehicle Trigger
  (bind _asbp_log_1 (Utilities|Casting|CastToBP_Log1 OtherActor)
    (:then
      (if (Variables|Default|GetRightBound)
        (Actor|DestroyActor _asbp_log_1)))
    (:CastFailed
      (bind _asbp_log_2 (Utilities|Casting|CastToBP_Log2 OtherActor))
      (if (Variables|Default|GetRightBound)
        (Actor|DestroyActor _asbp_log_2)))))

(event EventBeginPlay
  ;[1 1 1] Decides where the log is coming from
  (if (<= (Math|Random|RandomIntegerinRange 0 100) 50)
    (Variables|Default|SetLeftBound true) ; Car spawns on the right
    (Variables|Default|SetSpeed (Math|Random|RandomFloatinRange 1e+02 1.5e+02))
    (else
      (Variables|Default|SetRightBound true) ; Car spawns on the left
      (Variables|Default|SetSpeed (Math|Random|RandomFloatinRange 1e+02 1.5e+02)))))

(event EventTick
  (params (DeltaSeconds :type Float%20%28single-precision%29))
  ;[1 1 1] Spawn log at intervals between 0.25 sec and 3.0 sec
  (Utilities|FlowControl|Delay (Math|Random|RandomFloatinRange 1.4 2.0))
  (if (<= (Math|Random|RandomFloatinRange 0.0 1.0) 0.45)
    (CallFunction|SpawnLog1)
    (else
      (CallFunction|SpawnLog2))))

(fn ConstructionScript)

(fn SpawnLog1
  (bind _returnvalue (AddComponent|AddChildActorComponent false))
  (bind _asbp_log_1 (Utilities|Casting|CastToBP_Log1 (Variables|/Script/Engine.ChildActorComponent|GetChildActor _returnvalue)))
  (if (Variables|Default|GetLeftBound)
    (Variables|/Game/CrossyRoad/BluePrints/BP_Log1.BP_Log1_C|SetLogSpeed _asbp_log_1 (Variables|Default|GetSpeed))
    (Transformation|SetWorldTransform _returnvalue (Math|Transform|MakeTransform (Transformation|GetWorldLocation (Variables|Default|GetRightSpawn)) "0.000000,180.000000,0.000000" "1,1,1") false false)
    (else
      (Variables|/Game/CrossyRoad/BluePrints/BP_Log1.BP_Log1_C|SetLogSpeed _asbp_log_1 (Variables|Default|GetSpeed))
      (Transformation|SetWorldLocation _returnvalue (Transformation|GetWorldLocation (Variables|Default|GetLeftSpawn)) false false)
      (Transformation|SetWorldScale3D _returnvalue "1.000000,1.000000,1.000000"))))

(fn SpawnLog2
  (bind _returnvalue (AddComponent|AddChildActorComponent false))
  (bind _asbp_log_2 (Utilities|Casting|CastToBP_Log2 (Variables|/Script/Engine.ChildActorComponent|GetChildActor _returnvalue)))
  (if (Variables|Default|GetLeftBound)
    (Variables|/Game/CrossyRoad/BluePrints/BP_Log2.BP_Log2_C|SetLogSpeed _asbp_log_2 (Variables|Default|GetSpeed))
    (Transformation|SetWorldTransform _returnvalue (Math|Transform|MakeTransform (Transformation|GetWorldLocation (Variables|Default|GetRightSpawn)) "0.000000,180.000000,0.000000" "1,1,1") false false)
    (else
      (Variables|/Game/CrossyRoad/BluePrints/BP_Log2.BP_Log2_C|SetLogSpeed _asbp_log_2 (Variables|Default|GetSpeed))
      (Transformation|SetWorldLocation _returnvalue (Transformation|GetWorldLocation (Variables|Default|GetLeftSpawn)) false false)
      (Transformation|SetWorldScale3D _returnvalue "1.000000,1.000000,1.000000"))))