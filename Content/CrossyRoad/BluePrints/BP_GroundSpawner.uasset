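; Ground spawner for a Crossy Road-style game that builds a starting strip of random grass, road, track and river lanes.
; On BeginPlay it places grass under the player, then chains lanes through nested random rolls.
; Each lane spawns at the previous one's SpawnPoint, found through NewestWas flags, and receives a spawner reference.
; CheckLists would destroy all tracked lanes past MaxLanes, but its calls and the list tracking are disconnected.
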(event EventBeginPlay
  (CallFunction|SpawnInitialArea))

(event Collision|EventActorBeginOverlap
  (params (OtherActor :type Actor%20Object%20Reference)))

(event EventTick
  (params (DeltaSeconds :type Float%20%28single-precision%29)))

(fn ConstructionScript)

(fn SpawnGrassatSpawnPoint
  (params (SpawnLocation :type Vector))
  (bind _returnvalue (Game|SpawnActorfromClass "/Game/CrossyRoad/BluePrints/BP_SmallGrass.BP_SmallGrass_C" (Math|Transform|MakeTransform SpawnLocation "0, 0, 0" "1,1,1") "Undefined" 0 0))
  (bind _output_get (Variables|Default|SetNewestGrass _returnvalue))
  (Variables|/Game/CrossyRoad/BluePrints/BP_SmallGrass.BP_SmallGrass_C|SetGroundSpawner _output_get self)
  (return _returnvalue))

(fn SpawnatSpawnPoint
  (bind _returnvalue (Math|Random|RandomIntegerinRange 0 100))
  (if (< _returnvalue 30) ; 30% CHANCE FOR ROAD
    (bind _road_ref (CallFunction|SpawnRoad))
    (elif (< _returnvalue 31) ; 1% CHANCE FOR TRACKS
      (bind _trackref (CallFunction|SpawnTracks))
      (elif (< _returnvalue 32) ; 1% CHANCE FOR RIVER
        (bind _river_ref (CallFunction|SpawnRiver))
        (else
          (bind _grass_ref (CallFunction|SpawnGrass)))))))

(fn SpawnInitialArea
  (bind _returnvalue (Game|Player|GetPlayerPawn 0))
  (bind _returnvalue_2 (Transformation|GetActorLocation _returnvalue))
  (for _index (range 0 11)
    (Utilities|IsValid (Variables|Default|GetNewestGrass)
      (:Is%20Valid
        (CallFunction|SpawnatSpawnPoint))
      (:Is%20Not%20Valid
        (bind _grass_ref (CallFunction|SpawnGrassatSpawnPoint (Math|Vector|MakeVector (.x _returnvalue_2) (.y _returnvalue_2) (- (.z _returnvalue_2) 25.0))))))))

(fn SpawnRoadatSpawnPoint
  (params (SpawnLocation :type Vector))
  (bind _returnvalue (Game|SpawnActorfromClass "/Game/CrossyRoad/BluePrints/BP_SmallRoad.BP_SmallRoad_C" (Math|Transform|MakeTransform SpawnLocation "0, 0, 0" "1,1,1") "Undefined" 0 0))
  (bind _output_get (Variables|Default|SetNewestRoad _returnvalue))
  (Variables|/Game/CrossyRoad/BluePrints/BP_SmallRoad.BP_SmallRoad_C|SetGroundSpawner _output_get self)
  (return _returnvalue))

(fn SpawnTracksatSpawnPoint
  (params (SpawnLocation :type Vector))
  (bind _returnvalue (Game|SpawnActorfromClass "/Game/CrossyRoad/BluePrints/BP_Tracks.BP_Tracks_C" (Math|Transform|MakeTransform SpawnLocation "0, 0, 0" "1,1,1") "Undefined" 0 0))
  (bind _output_get (Variables|Default|SetNewestTracks _returnvalue))
  (Variables|/Game/CrossyRoad/BluePrints/BP_Tracks.BP_Tracks_C|SetGroundSpawner _output_get self)
  (return _returnvalue))

(fn SpawnGrass
  ;[1 1 1] Spawn Grass at appropriate spawn point (CHECK)
  (if (Variables|Default|GetNewestWasRoad)
    (bind _grass_ref (CallFunction|SpawnGrassatSpawnPoint (Transformation|GetWorldLocation (Variables|/Game/CrossyRoad/BluePrints/BP_SmallRoad.BP_SmallRoad_C|GetSpawnPoint (Variables|Default|GetNewestRoad)))))
    (Variables|Default|SetNewestWasRoad false)
    (Variables|Default|SetNewestWasTracks false)
    (Variables|Default|SetNewestWasRiver false)
    (return _grass_ref)
    (elif (Variables|Default|GetNewestWasTracks)
      (bind _grass_ref_2 (CallFunction|SpawnGrassatSpawnPoint (Transformation|GetWorldLocation (Variables|/Game/CrossyRoad/BluePrints/BP_Tracks.BP_Tracks_C|GetSpawnPoint (Variables|Default|GetNewestTracks)))))
      (Variables|Default|SetNewestWasTracks false)
      (Variables|Default|SetNewestWasRoad false)
      (Variables|Default|SetNewestWasRiver false)
      (return _grass_ref_2)
      (elif (Variables|Default|GetNewestWasRiver)
        (bind _grass_ref_3 (CallFunction|SpawnGrassatSpawnPoint (Transformation|GetWorldLocation (Variables|/Game/CrossyRoad/BluePrints/BP_SmallRiver.BP_SmallRiver_C|GetSpawnPoint (Variables|Default|GetNewestRiver)))))
        (Variables|Default|SetNewestWasTracks false)
        (Variables|Default|SetNewestWasRoad false)
        (Variables|Default|SetNewestWasRiver false)
        (return _grass_ref_3)
        (else
          (bind _grass_ref_4 (CallFunction|SpawnGrassatSpawnPoint (Transformation|GetWorldLocation (Variables|/Game/CrossyRoad/BluePrints/BP_SmallGrass.BP_SmallGrass_C|GetSpawnPoint (Variables|Default|GetNewestGrass)))))
          (Variables|Default|SetNewestWasTracks false)
          (Variables|Default|SetNewestWasRoad false)
          (Variables|Default|SetNewestWasRiver false)
          (return _grass_ref_4))))))

(fn SpawnRoad
  ;[1 1 1] Spawn Road at appropriate spawn point (CHECK)
  (if (Variables|Default|GetNewestWasRoad)
    (bind _road_ref (CallFunction|SpawnRoadatSpawnPoint (Transformation|GetWorldLocation (Variables|/Game/CrossyRoad/BluePrints/BP_SmallRoad.BP_SmallRoad_C|GetSpawnPoint (Variables|Default|GetNewestRoad)))))
    (Variables|Default|SetNewestWasRoad true)
    (Variables|Default|SetNewestWasTracks false)
    (Variables|Default|SetNewestWasRiver false)
    (return _road_ref)
    (elif (Variables|Default|GetNewestWasTracks)
      (bind _road_ref_2 (CallFunction|SpawnRoadatSpawnPoint (Transformation|GetWorldLocation (Variables|/Game/CrossyRoad/BluePrints/BP_Tracks.BP_Tracks_C|GetSpawnPoint (Variables|Default|GetNewestTracks)))))
      (Variables|Default|SetNewestWasRoad true)
      (Variables|Default|SetNewestWasTracks false)
      (Variables|Default|SetNewestWasRiver false)
      (return _road_ref_2)
      (elif (Variables|Default|GetNewestWasRiver)
        (bind _road_ref_3 (CallFunction|SpawnRoadatSpawnPoint (Transformation|GetWorldLocation (Variables|/Game/CrossyRoad/BluePrints/BP_SmallRiver.BP_SmallRiver_C|GetSpawnPoint (Variables|Default|GetNewestRiver)))))
        (Variables|Default|SetNewestWasRoad true)
        (Variables|Default|SetNewestWasTracks false)
        (Variables|Default|SetNewestWasRiver false)
        (return _road_ref_3)
        (else
          (bind _road_ref_4 (CallFunction|SpawnRoadatSpawnPoint (Transformation|GetWorldLocation (Variables|/Game/CrossyRoad/BluePrints/BP_SmallGrass.BP_SmallGrass_C|GetSpawnPoint (Variables|Default|GetNewestGrass)))))
          (Variables|Default|SetNewestWasRoad true)
          (Variables|Default|SetNewestWasTracks false)
          (Variables|Default|SetNewestWasRiver false)
          (return _road_ref_4))))))

(fn SpawnTracks
  ;[1 1 1] Spawn Tracks at appropriate spawn point (CHECK)
  (if (Variables|Default|GetNewestWasTracks)
    (bind _trackref (CallFunction|SpawnTracksatSpawnPoint (Transformation|GetWorldLocation (Variables|/Game/CrossyRoad/BluePrints/BP_Tracks.BP_Tracks_C|GetSpawnPoint (Variables|Default|GetNewestTracks)))))
    (Variables|Default|SetNewestWasTracks true)
    (Variables|Default|SetNewestWasRoad false)
    (Variables|Default|SetNewestWasRiver false)
    (return _trackref)
    (elif (Variables|Default|GetNewestWasRoad)
      (bind _trackref_2 (CallFunction|SpawnTracksatSpawnPoint (Transformation|GetWorldLocation (Variables|/Game/CrossyRoad/BluePrints/BP_SmallRoad.BP_SmallRoad_C|GetSpawnPoint (Variables|Default|GetNewestRoad)))))
      (Variables|Default|SetNewestWasTracks true)
      (Variables|Default|SetNewestWasRoad false)
      (Variables|Default|SetNewestWasRiver false)
      (return _trackref_2)
      (elif (Variables|Default|GetNewestWasRiver)
        (bind _trackref_3 (CallFunction|SpawnTracksatSpawnPoint (Transformation|GetWorldLocation (Variables|/Game/CrossyRoad/BluePrints/BP_SmallRiver.BP_SmallRiver_C|GetSpawnPoint (Variables|Default|GetNewestRiver)))))
        (Variables|Default|SetNewestWasTracks true)
        (Variables|Default|SetNewestWasRoad false)
        (Variables|Default|SetNewestWasRiver false)
        (return _trackref_3)
        (else
          (bind _trackref_4 (CallFunction|SpawnTracksatSpawnPoint (Transformation|GetWorldLocation (Variables|/Game/CrossyRoad/BluePrints/BP_SmallGrass.BP_SmallGrass_C|GetSpawnPoint (Variables|Default|GetNewestGrass)))))
          (Variables|Default|SetNewestWasTracks true)
          (Variables|Default|SetNewestWasRoad false)
          (Variables|Default|SetNewestWasRiver false)
          (return _trackref_4))))))

(fn SpawnRiveratSpawnPoint
  (params (SpawnLocation :type Vector))
  (bind _returnvalue (Game|SpawnActorfromClass "/Game/CrossyRoad/BluePrints/BP_SmallRiver.BP_SmallRiver_C" (Math|Transform|MakeTransform SpawnLocation "0, 0, 0" "1,1,1") "Undefined" 0 0))
  (bind _output_get (Variables|Default|SetNewestRiver _returnvalue))
  (Variables|/Game/CrossyRoad/BluePrints/BP_SmallRiver.BP_SmallRiver_C|SetGroundSpawner _output_get self)
  (return _returnvalue))

(fn SpawnRiver
  ;[1 1 1] Spawn River at appropriate spawn point (CHECK btw the branches are out of order, organize later)
  (if (Variables|Default|GetNewestWasRoad)
    (bind _river_ref (CallFunction|SpawnRiveratSpawnPoint (Transformation|GetWorldLocation (Variables|/Game/CrossyRoad/BluePrints/BP_SmallRoad.BP_SmallRoad_C|GetSpawnPoint (Variables|Default|GetNewestRoad)))))
    (Variables|Default|SetNewestWasRiver true)
    (Variables|Default|SetNewestWasTracks false)
    (Variables|Default|SetNewestWasRoad false)
    (return _river_ref)
    (elif (Variables|Default|GetNewestWasTracks)
      (bind _river_ref_2 (CallFunction|SpawnRiveratSpawnPoint (Transformation|GetWorldLocation (Variables|/Game/CrossyRoad/BluePrints/BP_Tracks.BP_Tracks_C|GetSpawnPoint (Variables|Default|GetNewestTracks)))))
      (Variables|Default|SetNewestWasRiver true)
      (Variables|Default|SetNewestWasTracks false)
      (Variables|Default|SetNewestWasRoad false)
      (return _river_ref_2)
      (elif (Variables|Default|GetNewestWasRiver)
        (bind _river_ref_3 (CallFunction|SpawnRiveratSpawnPoint (Transformation|GetWorldLocation (Variables|/Game/CrossyRoad/BluePrints/BP_SmallRiver.BP_SmallRiver_C|GetSpawnPoint (Variables|Default|GetNewestRiver)))))
        (Variables|Default|SetNewestWasRiver true)
        (Variables|Default|SetNewestWasTracks false)
        (Variables|Default|SetNewestWasRoad false)
        (return _river_ref_3)
        (else
          (bind _river_ref_4 (CallFunction|SpawnRiveratSpawnPoint (Transformation|GetWorldLocation (Variables|/Game/CrossyRoad/BluePrints/BP_SmallGrass.BP_SmallGrass_C|GetSpawnPoint (Variables|Default|GetNewestGrass)))))
          (Variables|Default|SetNewestWasRiver true)
          (Variables|Default|SetNewestWasTracks false)
          (Variables|Default|SetNewestWasRoad false)
          (return _river_ref_4))))))

(fn CheckLists
  (bind _roadlist (Variables|Default|GetRoadList))
  (bind _grasslist (Variables|Default|GetGrassList))
  (bind _trackslist (Variables|Default|GetTracksList))
  (bind _riverlist (Variables|Default|GetRiverList))
  (if (> (Variables|Default|GetLaneNum) (Variables|Default|GetMaxLanes))
    (for _array_element _grasslist
      (Actor|DestroyActor _array_element))
    (Utilities|Array|Clear _grasslist)
    (for _array_element_2 _roadlist
      (Actor|DestroyActor _array_element_2))
    (Utilities|Array|Clear _roadlist)
    (for _array_element_3 _trackslist
      (Actor|DestroyActor _array_element_3))
    (Utilities|Array|Clear _trackslist)
    (for _array_element_4 _riverlist
      (Actor|DestroyActor _array_element_4))
    (Utilities|Array|Clear _riverlist)
    (Variables|Default|SetLaneNum 0)))