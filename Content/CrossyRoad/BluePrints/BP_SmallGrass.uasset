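; BP_SmallGrass is a grass ground tile for a Crossy Road-style game, with randomly placed trees.
; On BeginPlay, SpawnTree runs for five spawn points, each with a roughly 30% chance of adding a scaled-up static mesh component there.
; When BP_Player enters the trigger zone, the tile tells its GroundSpawner to spawn at the spawn point.
; The GroundSpawner assignment and delayed self-destroy nodes are disconnected and never run.
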(event OnComponentBeginOverlap(Triggerzone)
  (params (OverlappedComponent :type Primitive%20Component%20Object%20Reference) (OtherActor :type Actor%20Object%20Reference) (OtherComp :type Primitive%20Component%20Object%20Reference) (OtherBodyIndex :type Integer) (bFromSweep :type Boolean) (SweepResult :type Hit%20Result%20Structure%20%28by%20ref%29))
  (Utilities|Casting|CastToBP_Player OtherActor)
  (Default|SpawnatSpawnPoint (Variables|Default|GetGroundSpawner)))

(event EventBeginPlay
  (Utilities|FlowControl|Sequence
    (:then_0
      (CallFunction|SpawnTree (Variables|Default|GetTreeSpawn1)))
    (:then_1
      (CallFunction|SpawnTree (Variables|Default|GetTreeSpawn2)))
    (:then_2
      (CallFunction|SpawnTree (Variables|Default|GetTreeSpawn3)))
    (:then_3
      (CallFunction|SpawnTree (Variables|Default|GetTreeSpawn4)))
    (:then_4
      (CallFunction|SpawnTree (Variables|Default|GetTreeSpawn5)))))

(fn ConstructionScript)

(fn SpawnTree
  (params (NewParam :type Scene%20Component%20Object%20Reference))
  (if (< (Math|Random|RandomIntegerinRange 0 100) 30)
    (bind _returnvalue (AddComponent|AddStaticMeshComponent false))
    (Transformation|SetWorldLocation _returnvalue (Transformation|GetWorldLocation NewParam) false false)
    (Transformation|SetWorldScale3D _returnvalue "2.500000,2.500000,2.500000")))